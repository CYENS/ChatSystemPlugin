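; Player controller component that provides a text chat for players to interact with performers during a performance.
; On the local controller it creates the chat widget, posts a welcome message and maps Enter and mouse wheel to focus and scroll.
; Messages pass through a server event that loops over the GameState PlayerArray, calling each controller's component to display them.
; A timer hides the chat after inactivity, cancelled while the chat is focused.
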(event `self.ReceiveBeginPlay`
  (if (`Controller.IsLocalPlayerController` (cast `PlayerController` (`self.GetOwner`) :!pure true))
    (bind _returnvalue (`|CreateWidget` "/ChatSystem/UI/WBP_ChatUI.WBP_ChatUI_C"))
    (bind _output_get (set `self.ChatUI` _returnvalue))
    (`UserWidget.AddToViewport` _output_get 0)
    (set `self.ChatBox` (`/ChatSystem/UI/WBP_ChatUI.WBP_ChatBox` _output_get))
    (add `/ChatSystem/UI/WBP_ChatBox.OnChatExit` (`self.ChatBox`) (delegate `OnChatExited`))
    (`/ChatSystem/UI/WBP_ChatBox.AddChatMessage` (`self.ChatBox`) "Welcome to this performance! \nPress Enter to write your messages and interract with the performers")
    (`self.HideChatAfterTime`)))

(event `OnChatExited`
  (`self.HideChatAfterTime`))

(event `Key|Enter`
  (params (Key :type "Key Structure"))
  (:`Pressed`
    (`/ChatSystem/UI/WBP_ChatBox.FocusChat` (`self.ChatBox`))))

(event `Key|MouseScrollUp`
  (params (Key :type "Key Structure"))
  (:`Pressed`
    (`/ChatSystem/UI/WBP_ChatBox.Scroll` (`self.ChatBox`) true)))

(event `Key|MouseScrollDown`
  (params (Key :type "Key Structure"))
  (:`Pressed`
    (`/ChatSystem/UI/WBP_ChatBox.Scroll` (`self.ChatBox`) false)))

(event `SendChatMessageOnServer`
  (params (Message :type String))
  (for _array_element (`GameStateBase.PlayerArray` (`GameplayStatics.GetGameState`))
    (`self.AddChatMessageOnOwningClient` (`Actor.GetComponentByClass` (`PlayerState.GetPlayerController` _array_element) "BP_ChatSystemComponent_C") Message)))

(event `AddChatMessageOnOwningClient`
  (params (Message :type String))
  (`/ChatSystem/UI/WBP_ChatBox.AddChatMessage` (`self.ChatBox`) Message)
  (`self.HideChatAfterTime`))

(event `HideChatAfterTime`
  (bind _returnvalue (`KismetSystemLibrary.K2_SetTimerDelegate` (delegate `TimerFinished`) (`self.SecondsUntilHidingChat`)))
  ;[1 1 1] Don't hide if chat is focused
  (add `/ChatSystem/UI/WBP_ChatBox.OnChatFocus` (`self.ChatBox`) (delegate `ChatFocused`)))

(event `ChatFocused`
  ;[1 1 1] Don't hide if chat is focused
  (`KismetSystemLibrary.K2_ClearAndInvalidateTimerHandle` (stale `HideChatAfterTime` _returnvalue)))

(event `TimerFinished`
  (`self.HideChatIfNotFocused`))

(fn `HideChatIfNotFocused`
  (if (not (`/ChatSystem/UI/WBP_ChatBox.isFocused` (`self.ChatBox`)))
    (`/ChatSystem/UI/WBP_ChatBox.HideChat` (`self.ChatBox`))))