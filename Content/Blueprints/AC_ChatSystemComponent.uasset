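; Player controller component that provides multiplayer text chat with an auto-hiding chat box.
; On the local controller it creates WBP_ChatUI, shows an optional welcome message and binds to the chat box's entry, focus and exit events.
; Entered text gets the player's name prepended, then SendChatMessageOnServer relays it to the component on every PlayerArray controller.
; Incoming messages reveal the box and restart its hide timer, which focusing cancels.
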(event `self.ReceiveBeginPlay`
  (bind _welcome_message (`self.Welcome Message`))
  (if (`Controller.IsLocalPlayerController` (cast `PlayerController` (`self.GetOwner`) :!pure true))
    (bind _returnvalue (`|CreateWidget` "/ChatSystem/UI/WBP_ChatUI.WBP_ChatUI_C"))
    (bind _output_get (set `self.ChatUI` _returnvalue))
    (`UserWidget.AddToViewport` _output_get 0)
    (set `self.ChatBox` (`/ChatSystem/UI/WBP_ChatUI.WBP_ChatBox` _output_get))
    (add `/ChatSystem/UI/WBP_ChatBox.OnChatExit` (`self.ChatBox`) (delegate `OnChatExitedEvent`))
    (add `/ChatSystem/UI/WBP_ChatBox.OnMessageEntered` (`self.ChatBox`) (delegate `OnMessageEntered`))
    (`|ExecutionSequence`
      (:`then_0`
        (if (not (`KismetStringLibrary.IsEmpty` _welcome_message))
          (`/ChatSystem/UI/WBP_ChatBox.AddChatMessage` (`self.ChatBox`) _welcome_message)))
      (:`then_1`
        (`self.HideChatAfterTime`)))))

(event `OnChatExitedEvent`
  (`self.HideChatAfterTime`))

(event `OnMessageEntered`
  (params (Message :type String))
  (`|ExecutionSequence`
    (:`then_0`
      (if (not (`KismetStringLibrary.IsEmpty` Message))
        (`self.SendChatMessageOnServer` (`KismetStringLibrary.Concat_StrStr` (`PlayerState.GetPlayerName` (`Controller.PlayerState` (`GameplayStatics.GetPlayerController` 0))) ": " Message))))
    (:`then_1`
      (`self.ExitChat`))))

(event `SendChatMessageOnServer`
  (params (Message :type String))
  (for _array_element (`GameStateBase.PlayerArray` (`GameplayStatics.GetGameState`))
    (`self.AddChatMessageOnOwningClient` (`Actor.GetComponentByClass` (`PlayerState.GetPlayerController` _array_element) "AC_ChatSystemComponent_C") Message)))

(event `AddChatMessageOnOwningClient`
  (params (Message :type String))
  (`/ChatSystem/UI/WBP_ChatBox.ShowChat` (`self.ChatBox`))
  (`/ChatSystem/UI/WBP_ChatBox.AddChatMessage` (`self.ChatBox`) Message)
  (`KismetSystemLibrary.K2_ClearAndInvalidateTimerHandle` (`self.CurrentVisibilityTimer`))
  (`self.HideChatAfterTime`))

(event `HideChatAfterTime`
  (bind _returnvalue (`KismetSystemLibrary.K2_SetTimerDelegate` (delegate `TimerFinished`) (`self.SecondsUntilHidingChat`)))
  ;[1 1 1] Don't hide if chat is focused
  (add `/ChatSystem/UI/WBP_ChatBox.OnChatFocus` (`self.ChatBox`) (delegate `ChatFocused`))
  (set `self.CurrentVisibilityTimer` _returnvalue))

(event `ChatFocused`
  ;[1 1 1] Don't hide if chat is focused
  (`KismetSystemLibrary.K2_ClearAndInvalidateTimerHandle` (stale `HideChatAfterTime` _returnvalue)))

(event `TimerFinished`
  (`self.HideChatIfNotFocused`))

(fn `ExitChat`
  (`/ChatSystem/UI/WBP_ChatBox.ExitChat` (`self.ChatBox`)))

(fn `FocusChat`
  (`/ChatSystem/UI/WBP_ChatBox.FocusChat` (`self.ChatBox`)))

(fn `HideChatIfNotFocused`
  (if (not (`/ChatSystem/UI/WBP_ChatBox.isFocused` (`self.ChatBox`)))
    (`/ChatSystem/UI/WBP_ChatBox.HideChat` (`self.ChatBox`))))

(fn `ScrollDown`
  (`/ChatSystem/UI/WBP_ChatBox.Scroll` (`self.ChatBox`) false))

(fn `ScrollUp`
  (`/ChatSystem/UI/WBP_ChatBox.Scroll` (`self.ChatBox`) true))