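; Player controller that routes Enhanced Input to a chat system component.
; On BeginPlay it adds the chat input mapping context to the local player's Enhanced Input subsystem, if that subsystem is valid.
; The focus action focuses the chat, and the scroll action scrolls it up or down by the sign of its value.
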(event `self.ReceiveBeginPlay`
  (bind _returnvalue (subsystem `EnhancedInputLocalPlayerSubsystem`))
  (`/Engine/EditorBlueprintResources/StandardMacros.IsValid` _returnvalue
    (:`Is Valid`
      (`EnhancedInputSubsystemInterface.AddMappingContext` _returnvalue "/ChatSystem/Input/IMC_ChatSystem.IMC_ChatSystem" 0 (struct)))))

(event `EnhancedInput|/ChatSystem/Input/IA_FocusChat`
  (params (ActionValue :type Boolean) (ElapsedSeconds :type "Float (double-precision)") (TriggeredSeconds :type "Float (double-precision)") (InputAction :type "InputAction Object Reference" :default "/ChatSystem/Input/IA_FocusChat.IA_FocusChat"))
  (:`Triggered`
    (`/ChatSystem/Blueprints/BP_ChatSystemComponent.FocusChat` (`self.BP_ChatSystemComponent`))))

(event `EnhancedInput|/ChatSystem/Input/IA_ScrollChat`
  (params (ActionValue :type "Float (double-precision)") (ElapsedSeconds :type "Float (double-precision)") (TriggeredSeconds :type "Float (double-precision)") (InputAction :type "InputAction Object Reference" :default "/ChatSystem/Input/IA_ScrollChat.IA_ScrollChat"))
  (:`Triggered`
    (if (> ActionValue 0.0)
      (`/ChatSystem/Blueprints/BP_ChatSystemComponent.ScrollUp` (`self.BP_ChatSystemComponent`))
      (else
        (`/ChatSystem/Blueprints/BP_ChatSystemComponent.ScrollDown` (`self.BP_ChatSystemComponent`))))))

(fn `UserConstructionScript`)